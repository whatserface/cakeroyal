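; Rifle weapon Blueprint that supplies the recoil response when the gun fires.
; Recoil adds a random one-directional pitch kick and a small random yaw drift to the target's controller input.
; It then plays the first-person rifle fire montage on a BP_PlayerCharacter's InnerMesh, or prints a debug string when that cast fails.
; RedoRecoil is a stub that only checks target validity.
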(event `self.Recoil`
  (params (ApplyTo :type "Pawn Object Reference"))
  (`/Engine/EditorBlueprintResources/StandardMacros.IsValid` ApplyTo
    (:`Is Valid`
      (`Pawn.AddControllerPitchInput` ApplyTo (`KismetMathLibrary.RandomFloatInRange` -0.1 -0.5))
      (`Pawn.AddControllerYawInput` ApplyTo (`KismetMathLibrary.RandomFloatInRange` -0.2 0.2))
      (bind _asbp_player_character (cast `/Game/Blueprints/Character/BP_PlayerCharacter` ApplyTo)
        (:`then`
          (`|PlayMontage` (`PlayerCharacter.InnerMesh` _asbp_player_character) "/Game/Animations/FPP_Animations/HerroFPP_RifleFire_Montage.HerroFPP_RifleFire_Montage"))
        (:`CastFailed`
          (`KismetSystemLibrary.PrintString` "Hello"))))))

(event `self.Redo_Recoil`
  (params (ApplyTo :type "Pawn Object Reference"))
  (`/Engine/EditorBlueprintResources/StandardMacros.IsValid` ApplyTo))

(fn `UserConstructionScript`)