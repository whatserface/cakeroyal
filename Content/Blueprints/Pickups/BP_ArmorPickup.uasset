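; BP_ArmorPickup is a pickup that grants armor to the actor that collects it.
; It overrides GivePickupto to find that actor's HealthComponent and try to add the ArmorToAdd amount.
; Its ShouldBother override allows pickup only when the parent check passes, a HealthComponent exists and its armor is not already full.
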(event `self.GivePickupTo`
  (params (PickupActor :type "Actor Object Reference"))
  (bind _returnvalue (`self.GetComponentByClass` PickupActor "/Script/pettest.HealthComponent"))
  (`/Engine/EditorBlueprintResources/StandardMacros.IsValid` _returnvalue
    (:`Is Valid`
      (`HealthComponent.TryToAddArmor` _returnvalue (`self.ArmorToAdd`)))))

(fn `ShouldBother`
  (params (PickupActor :type "Actor Object Reference"))
  (returns (bBother :type Boolean))
  (bind _returnvalue (`self.GetComponentByClass` PickupActor "/Script/pettest.HealthComponent"))
  (`/Engine/EditorBlueprintResources/StandardMacros.IsValid` _returnvalue
    (:`Is Valid`
      (return (and (`parent.ShouldBother` PickupActor) (not (`HealthComponent.IsArmorFull` _returnvalue)))))
    (:`Is Not Valid`
      (return false))))

(fn `UserConstructionScript`
  (`parent.UserConstructionScript`))