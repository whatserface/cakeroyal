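; BP_GameModeBase is a game mode Blueprint whose only active logic is what looks like a debug check on player characters.
; Two seconds after BeginPlay, it picks random player indices from the player count and looks up their controlled pawns.
; If the pawn is a valid BP_PlayerCharacter, it prints whether that character's InnerMesh is visible.
; Tick and the construction script are empty.
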(event `self.ReceiveBeginPlay`
  (`KismetSystemLibrary.Delay` 2.0)
  (bind _returnvalue (`self.GetNumPlayers`))
  (bind _returnvalue_2 (`Controller.K2_GetPawn` (`GameplayStatics.GetPlayerController` (`KismetMathLibrary.RandomInteger` _returnvalue))))
  (`/Engine/EditorBlueprintResources/StandardMacros.IsValid` _returnvalue_2
    (:`Is Valid`
      (bind _asbp_player_character (cast `/Game/Blueprints/Character/BP_PlayerCharacter` _returnvalue_2))
      (`/Engine/EditorBlueprintResources/StandardMacros.IsValid` _asbp_player_character
        (:`Is Valid`
          (`KismetSystemLibrary.PrintString` (`KismetStringLibrary.Conv_BoolToString` (`SceneComponent.IsVisible` (`PlayerCharacter.InnerMesh` _asbp_player_character)))))))))

(fn `UserConstructionScript`)